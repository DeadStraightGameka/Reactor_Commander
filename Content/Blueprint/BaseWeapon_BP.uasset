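; Base weapon Blueprint that provides two firing functions, hitscan energy and spawned projectile, both originating from a socket on the gun mesh.
; ShootEnergy line-traces on the Camera channel, spawns an impact emitter, then applies and prints damage read from the hardcoded PlasmaGun row of the WeaponSlot data table.
; ShootProjectile spawns a projectile at the socket transform, ignoring its EndLocation input.
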(event EventBeginPlay)

(event Collision|EventActorBeginOverlap
  (params (OtherActor :type Actor%20Object%20Reference)))

(event EventTick
  (params (DeltaSeconds :type Float%20%28single-precision%29)))

(fn ConstructionScript)

(fn ShootEnergy
  (params (StartLocation :type Name) (EndLocation :type Vector))
  (bind (_outhit _returnvalue) (Collision|LineTraceByChannel (.Location (Math|Transform|BreakTransform (Transformation|GetSocketTransform (Variables|Default|GetGunMesh01) StartLocation "RTS_World"))) EndLocation "TraceTypeQuery2" true 0 "None"))
  (if _returnvalue
    (Effects|SpawnEmitteratLocation "/Engine/Tutorial/SubEditors/TutorialAssets/TutorialParticleSystem.TutorialParticleSystem" (.Location (Collision|BreakHitResult _outhit)))
    (bind _returnvalue_2 (Utilities|GetDataTableRow "/Game/Jimmy_Test/WeaponSlot.WeaponSlot" "PlasmaGun")
      (:then
        (bind _returnvalue_3 (Game|Damage|ApplyDamage (.HitActor (Collision|BreakHitResult _outhit)) (.Damage (Utilities|Struct|BreakWeaponStat _returnvalue_2)) 0 0))
        (Development|PrintString (Utilities|String|ToString(Float) _returnvalue_3))))))

(fn ShootProjectile
  (params (WeaponSocket :type Name) (EndLocation :type Vector))
  (Game|SpawnActorfromClass "/Game/Blueprint/Projectile.Projectile_C" (Transformation|GetSocketTransform (Variables|Default|GetGunMesh01) WeaponSocket "RTS_World") "AlwaysSpawn" 0 0))