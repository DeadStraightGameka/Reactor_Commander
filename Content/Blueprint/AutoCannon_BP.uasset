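; AutoCannon_BP is an auto cannon weapon Blueprint that initializes its combat stats from data.
; On BeginPlay it reads the BalisticGun row of the WeaponSlot data table into Damage, MaxBulletDistance and RateofFire, then prints them for debugging.
; It contains no firing logic of its own, and its construction script only calls the parent's.
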(event EventBeginPlay
  (bind _returnvalue (Utilities|GetDataTableRow "/Game/Jimmy_Test/WeaponSlot.WeaponSlot" "BalisticGun")
    (:then
      (bind _output_get (Variables|Default|SetDamage (.Damage (Utilities|Struct|BreakWeaponStat _returnvalue))))
      (bind _output_get_2 (Variables|Default|SetMaxBulletDistance (.MaxBulletDistance (Utilities|Struct|BreakWeaponStat _returnvalue))))
      (bind _output_get_3 (Variables|Default|SetRateofFire (.RateofFire (Utilities|Struct|BreakWeaponStat _returnvalue))))
      (Development|PrintString (Utilities|String|Append "Damage: " (Utilities|String|ToString(Float) _output_get) "MaxDistance: " (Utilities|String|ToString(Float) _output_get_2) "Rate Of Fire: " (Utilities|String|ToString(Float) _output_get_3))))))

(event Collision|EventActorBeginOverlap
  (params (OtherActor :type Actor%20Object%20Reference)))

(event EventTick
  (params (DeltaSeconds :type Float%20%28single-precision%29)))

(fn ConstructionScript
  (|CallParentFunction))