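; HUD Blueprint that creates the gameplay widget and relays kill notifications and match results to it.
; On BeginPlay it creates GameplayHUD, hands it a self reference and adds it to the viewport.
; It retries every 0.2 seconds until the owning controller's PlayerState casts to PlayerStateBP, then binds its kill and result handlers.
; Those handlers forward events through CallShowAKill and CallShowResult dispatchers.
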(event Custom|ReceivedResult
  (params (Win :type Boolean))
  (Default|CallShowResult Win))

(event Custom|ReceivedKillNotify
  (params (Killer :type Text) (Victim :type Text))
  ;[1 1 1] Pass information to everyone
  (Default|CallShowAKill Killer Victim))

(event EventBeginPlay
  (bind _returnvalue (Game|Player|GetOwningPlayerController))
  ;[1 1 1] Pass information to everyone
  (bind _returnvalue_2 (UserInterface|CreateWidget "/Game/UI/AllLevels/GameplayHUD.GameplayHUD_C" _returnvalue 0))
  (bind _output_get (Variables|Default|SetGameplayHUD _returnvalue_2))
  (Variables|/Game/UI/AllLevels/GameplayHUD.GameplayHUD_C|SetourHUD _output_get self)
  (UserInterface|Viewport|AddtoViewport _returnvalue_2 0)
  (bind _asplayer_state_bp (Utilities|Casting|CastToPlayerStateBP (Variables|/Script/Engine.Controller|GetPlayerState _returnvalue) :!label _label)
    (:then
      (EventDispatchers|BindEventtoReceiveKillNotify _asplayer_state_bp (delegate Custom|ReceivedKillNotify))
      (EventDispatchers|BindEventtoReceiveResult _asplayer_state_bp (delegate Custom|ReceivedResult)))
    (:CastFailed
      (Utilities|FlowControl|Delay 0.2)
      (goto _label))))

(fn ConstructionScript)