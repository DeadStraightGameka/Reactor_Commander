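; Twin-turret gun drone demo Blueprint for the AI Turret Controller.
; Each tick it spins seven fan meshes in yaw at a frame-rate-independent rate set by FanRotationsPerSecond.
; The construction script appends the landing gear mesh to the turret controller's ignore list so it cannot block target finding, adding rather than setting to keep the controller's default entries.
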(event EventTick
  (params (DeltaSeconds :type Float%20%28single-precision%29))
  ;[1 1 1] Spin The Fans
  (Transformation|AddLocalRotation (Variables|Default|GetGD_Fan_Mesh2) (Math|Rotator|MakeRotator 0.0 0.0 (* (Utilities|Time|GetWorldDeltaSeconds) (Variables|Default|GetFan%20Rotations%20Per%20Second) 3.6e+02)) false false))

(fn ConstructionScript
  ;[1 1 1] Keep the landing gear from obstructing the turrets ability to find targets, since the gear would just rotate with the turret and never end up in the guns path anyway. It's important to add and not set, or you'll overwrite some default additions made by the controller.
  (Utilities|Array|Add (Variables|/Game/AI_Turret_Controller/Blueprints/AI_Turret_Controller_BP/AI_Turret_Controller_BP.AI_Turret_Controller_BP_C|GetComponents%20To%20Ignore (Variables|Default|GetAI_Turret_Controller)) (Variables|Default|GetGD_Landing_Rods_Mesh)))