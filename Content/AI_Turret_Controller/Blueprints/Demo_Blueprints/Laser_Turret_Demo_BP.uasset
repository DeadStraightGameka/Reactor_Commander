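; Demo laser turret actor built on the AI Turret Controller component, with an animated turret ball and an optional forced-fire mode.
; Firing changes are replicated from the authority to drive spin-up, firing and spin-down animations, using delays and state flags to avoid overlaps.
; A looping timeline bobs the turret up and down.
; The construction script adds the ball mesh to the controller's ignore list so it can spot targets through it.
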(event Custom|Update%20Firing%20%28replicated%29
  (params (Condition :type Boolean))
  (bind _turret_ball (Variables|Default|GetTurret_Ball))
  ;[1 1 1] Set The Current Animation For Firing
  (if Condition
    (if (not (Variables|Default|GetSpun%20Up))
      (if (not (Variables|Default|GetSpinning%20Up))
        (Components|Animation|OverrideAnimationData _turret_ball "/Game/AI_Turret_Controller/Animations/LT_Ball_Start.LT_Ball_Start" true true 0.0 1.0)
        (Variables|Default|SetSpinning%20Up true)
        (Utilities|FlowControl|Delay 1.198)
        (Variables|Default|SetSpinning%20Up false)
        (Components|Animation|OverrideAnimationData _turret_ball "/Game/AI_Turret_Controller/Animations/LT_Ball_Firing.LT_Ball_Firing" true true 0.0 1.0)
        (Variables|Default|SetSpun%20Up true)))
    (elif (Variables|Default|GetSpun%20Up)
      (if (not (Variables|Default|GetSpinning%20Down))
        (Variables|Default|SetSpinning%20Down true)
        (Components|Animation|OverrideAnimationData _turret_ball "/Game/AI_Turret_Controller/Animations/LT_Ball_Stop.LT_Ball_Stop" true true 0.0 1.0)
        (Utilities|FlowControl|Delay 1.198)
        (Variables|Default|SetSpinning%20Down false)
        (Variables|Default|SetSpun%20Up false)
        (Components|Animation|OverrideAnimationData _turret_ball "/Game/AI_Turret_Controller/Animations/LT_Ball_Stopped.LT_Ball_Stopped" false true 0.0 1.0)))))

(event EventBeginPlay
  (Utilities|FlowControl|Sequence
    (:then_0
      ;[1 1 1] Move A Target Up And Down Over Time
      (bind (_direction _track1) (Timeline|Timeline_0 PlayFromStart)
        (:Update
          (Transformation|SetRelativeLocation (Variables|Default|GetTurret1) (Math|Vector|MakeVector 0.0 0.0 (* _track1 (Variables|Default|GetBob_Multiplier))) false false))
        (:Finished
          (if (Utilities|Enum|Equal(Enum) _direction "Forward")
            (Timeline|Timeline_0 Reverse)
            (else
              (Timeline|Timeline_0 Play))))))
    (:then_1
      ;[1 1 1] Sets the laser turret to force fire if enabled
      (if (Variables|Default|GetForced%20Fire%20Enabled)
        (Default|ForceTurrettoFire(Laser) (Variables|Default|GetAI_Turret_Controller%20%28Main%20turret%29) true)))))

(event EventTurretFiring
  (params (Fired%20Projectile :type Actor%20Object%20Reference) (Emitter%20Firing :type Actor%20Component%20Object%20Reference) (Firing%20At :type Actor%20Object%20Reference) (Firing%20At%20Component :type Scene%20Component%20Object%20Reference) (Parent%20Controller :type AI%20Turret%20Controller%20BP%20Object%20Reference) (Firing :type Boolean) (Forced%20FIring :type Boolean))
  ;[1 1 1] Set The Current Animation For Firing
  (Networking|SwitchHasAuthority
    (:Authority
      (CallFunction|UpdateFiring(replicated) Firing))))

(fn ConstructionScript
  ;[1 1 1] Add Skeletal Component To Ignore List So Main Turret Can Spot Enemies Through Them. If Ignore Self Was Enabled This Woudn't Be Needed, But Its Good To Know How To Do This If You Dont Want Your Turret To Spot Targets Through All Parts Of The Actor (Like A Battleship Cannon Seeing Enemis Through The Command Tower)
  (Utilities|Array|Add (Variables|/Game/AI_Turret_Controller/Blueprints/AI_Turret_Controller_BP/AI_Turret_Controller_BP.AI_Turret_Controller_BP_C|GetComponents%20To%20Ignore (Variables|Default|GetAI_Turret_Controller%20%28Main%20turret%29)) (Variables|Default|GetTurret_Ball)))