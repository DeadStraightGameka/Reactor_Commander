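; Continuous laser actor for the AI turret demo that draws a beam from a turret's emitter to its target while firing.
; Begin and end fire events store the target and toggle beam visibility and Tick, which moves the beam endpoints each frame.
; On BeginPlay, non-server instances call events meant to sync visibility and tick state from the server.
; It is visual only, with damage left as a noted extension point.
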(event Custom|Set%20Status%20Clients
  (params (bNewVisibility :type Boolean) (bEnabled :type Boolean))
  ;[1 1 1] Update beam status on start from server
  (Rendering|SetVisibility (Variables|Default|GetP_Beam_Laser) bNewVisibility false)
  (Actor|Tick|SetActorTickEnabled bEnabled))

(event Custom|Get%20Status%20from%20server
  ;[1 1 1] Update beam status on start from server
  (CallFunction|SetStatusClients (Variables|/Script/Engine.SceneComponent|GetbVisible (Variables|Default|GetP_Beam_Laser)) (Class|Actor|IsActorTickEnabled)))

(event EventContinuousLaserSpawn
  (params (Parent%20Controller :type AI%20Turret%20Controller%20BP%20Object%20Reference) (Parent%20Emitter :type Scene%20Component%20Object%20Reference))
  (Variables|Default|SetParent%20Emitter Parent%20Emitter))

(event EventTick
  (params (DeltaSeconds :type Float%20%28single-precision%29))
  ;[1 1 1] When Firing, Point Beam At Targets Location. You'd Want To Apply Damage After Here Too Normally.
  (if (Variables|Default|GetFiring)
    (Class|ParticleSystemComponent|SetBeamSourcePoint (Variables|Default|GetP_Beam_Laser) 0 (Transformation|GetWorldLocation (Variables|Default|GetParent%20Emitter)))
    (Class|ParticleSystemComponent|SetBeamEndPoint (Variables|Default|GetP_Beam_Laser) 0 (Transformation|GetWorldLocation (Variables|Default|GetTarget_Component)))))

(event EventBeginPlay
  ;[1 1 1] Update beam status on start from server
  (if (not (Networking|IsServer))
    (CallFunction|GetStatusfromServer)))

(event EventContinuousLaserBeginFire
  (params (Firing%20At :type Actor%20Object%20Reference) (Firing%20At%20Component :type Scene%20Component%20Object%20Reference) (Aiming%20At%20Location :type Vector :default "0, 0, 0") (Current%20Ammo :type Integer) (Damage%20Multiplier :type Float%20%28single-precision%29) (Forced%20Fire :type Boolean))
  ;[1 1 1] Get Information On When To Or Not Too Fire
  (Variables|Default|SetTarget Firing%20At)
  (Variables|Default|SetTarget_Component Firing%20At%20Component)
  (Variables|Default|SetFiring true)
  (Actor|Tick|SetActorTickEnabled true)
  (Rendering|SetVisibility (Variables|Default|GetP_Beam_Laser) true false))

(event EventContinuousLaserEndFire
  (params (Firing%20At :type Actor%20Object%20Reference) (Firing%20At%20Component :type Scene%20Component%20Object%20Reference) (Aiming%20At%20Location :type Vector :default "0, 0, 0") (Current%20Ammo :type Integer) (Damage%20Multiplier :type Float%20%28single-precision%29))
  ;[1 1 1] Get Information On When To Or Not Too Fire
  (Variables|Default|SetTarget Firing%20At)
  (Variables|Default|SetTarget_Component Firing%20At%20Component)
  (Variables|Default|SetFiring false)
  (Actor|Tick|SetActorTickEnabled false)
  (Rendering|SetVisibility (Variables|Default|GetP_Beam_Laser) false false))

(fn ConstructionScript)