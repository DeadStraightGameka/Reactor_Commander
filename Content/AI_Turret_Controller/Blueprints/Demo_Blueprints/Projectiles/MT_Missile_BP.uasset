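; Homing missile projectile for the AI turret demo, which flies at a target actor and component handed to it at launch.
; After an arming delay, Tick turns it toward the component's center of mass or pivot and eases forward physics velocity toward missile speed.
; It explodes on hit, lifetime expiry, or proximity to "Fire_At" components on tagged actors.
; The server multicasts the explosion effect and destruction; no damage is applied.
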(event OnComponentHit(Missile)
  (params (HitComponent :type Primitive%20Component%20Object%20Reference) (OtherActor :type Actor%20Object%20Reference) (OtherComp :type Primitive%20Component%20Object%20Reference) (NormalImpulse :type Vector :default "0, 0, 0") (Hit :type Hit%20Result%20Structure%20%28by%20ref%29))
  ;[1 1 1] On Hit Or Explode, You'd Add Damage Dealt Here
  (if (!= HitComponent (Components|GetOwner))
    (if (Networking|IsServer)
      (CallFunction|Explode(multicast) (Transformation|GetWorldLocation (Variables|Default|GetMissile))))))

(event Custom|Explode%20%28multicast%29
  (params (Location :type Vector))
  ;[1 1 1] On Hit Or Explode, You'd Add Damage Dealt Here
  (Effects|SpawnEmitteratLocation "/Game/AI_Turret_Controller/Particles/Explosion_P.Explosion_P" Location "0, 0, 0" "3.500000,3.500000,3.500000" false)
  (Actor|DestroyActor))

(event Custom|Explode
  ;[1 1 1] On Hit Or Explode, You'd Add Damage Dealt Here
  (if (Networking|IsServer)
    (CallFunction|Explode(multicast) (Transformation|GetWorldLocation (Variables|Default|GetMissile)))))

(event EventBeginPlay
  (bind _missile (Variables|Default|GetMissile))
  ;[1 1 1] Set Initial Missile Speed
  (Physics|SetPhysicsLinearVelocity _missile (+ (Transformation|GetVelocity (Components|GetOwner)) (Math|Vector|RotateVector (Math|Vector|MakeVector (* (Variables|Default|GetMissile%20Speed) 0.5) 0.0 0.0) (Transformation|GetWorldRotation _missile))) false "None")
  ;[1 1 1] Set Delays For Missile Guidance And Death
  (Utilities|FlowControl|Delay (Variables|Default|GetTarget%20Delay))
  (Variables|Default|SetArmed true)
  (Utilities|FlowControl|Delay (Variables|Default|GetMissile%20Life))
  (CallFunction|Explode))

(event EventTick
  (params (DeltaSeconds :type Float%20%28single-precision%29))
  (bind _returnvalue (Utilities|Time|GetWorldDeltaSeconds))
  (bind _returnvalue_2 (Transformation|GetActorRotation))
  (bind _missile (Variables|Default|GetMissile))
  (bind _missile_2 (Variables|Default|GetMissile))
  (bind _target (Variables|Default|GetTarget))
  (bind _missile_3 (Variables|Default|GetMissile))
  (bind _returnvalue_3 (Transformation|GetWorldLocation _missile))
  ;[1 1 1] If Armed And Target Is Valid Aim Towards It, If Not Just Fly Straight
  (if (Variables|Default|GetArmed)
    (Utilities|FlowControl|Sequence
      (:then_0
        ;[1 1 1] Get All Hostile Actors
        (bind _outactors (Actor|GetAllActorswithTag (Variables|Default|GetTarget%20Tag)))
        ;[1 1 1] Check For Target Components Within Range Of Missile
        (for _array_element _outactors
          (for _array_element_2 (Actor|GetComponentsbyTag _array_element "/Script/Engine.SceneComponent" "Fire_At")
            (if (<= (Math|Vector|VectorLength (- (Transformation|GetWorldLocation _array_element_2) (Transformation|GetActorLocation))) (Variables|Default|GetProximity%20Fuse%20Range))
              (CallFunction|Explode)))))
      (:then_1
        (Utilities|IsValid self
          (:Is%20Valid
            (if (== 0 _target)
              _
              (else
                (Utilities|IsValid _target
                  (:Is%20Valid
                    ;[1 1 1] If Target Component Is Primitive Aim For Center Of Mass, If Not Aim For Pivot Point (Pivots On Many Meshes Are Bellow The Actual Mesh, So This Is Useful Depending On Your Art Assets)
                    (bind _asprimitive_component (Utilities|Casting|CastToPrimitiveComponent (Variables|Default|GetTarget%20Component))
                      (:then
                        (if (Math|Vector|Equal(Vector) (Physics|GetCenterOfMass _asprimitive_component "None") "0, 0, 0" 0.0001)
                          (Transformation|SetActorRotation (Class|KismetMathLibrary|RInterptoConstant _returnvalue_2 (Math|Rotator|FindLookatRotation _returnvalue_3 (Transformation|GetWorldLocation (Variables|Default|GetTarget%20Component))) _returnvalue 3.1e+02) true :!label _label)
                          (else
                            (Transformation|SetActorRotation (Class|KismetMathLibrary|RInterptoConstant _returnvalue_2 (Math|Rotator|FindLookatRotation _returnvalue_3 (Physics|GetCenterOfMass _asprimitive_component "None")) _returnvalue 3.1e+02) true))))
                      (:CastFailed
                        (goto _label))))
                  (:Is%20Not%20Valid
                    _))))
            ;[1 1 1] Set Missile Speed
            (Physics|SetPhysicsLinearVelocity _missile_3 (Math|Vector|RotateVector (Math|Vector|MakeVector (Math|Interpolation|FInterptoConstant (.x (Math|Vector|UnrotateVector (Transformation|GetComponentVelocity _missile_2) (Transformation|GetWorldRotation _missile_2))) (Variables|Default|GetMissile%20Speed) (Utilities|Time|GetWorldDeltaSeconds) (Variables|Default|GetAccel%20Decell%20rate)) 0.0 0.0) (Transformation|GetWorldRotation _missile_3)) false "None")))))))

(event EventProjectileTarget
  (params (Targeted%20Actor :type Actor%20Object%20Reference) (Firing%20At%20Component :type Scene%20Component%20Object%20Reference) (Aim%20At%20Location :type Vector :default "0, 0, 0") (Parent%20ControllerParent%20Controller :type AI%20Turret%20Controller%20BP%20Object%20Reference) (Damage%20Multiplier :type Float%20%28single-precision%29))
  ;[1 1 1] Get Target Information
  (Variables|Default|SetTarget Targeted%20Actor)
  (Variables|Default|SetTarget%20Component Firing%20At%20Component))

(fn ConstructionScript)