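; CT_Projectile_BP is a demo projectile for the AI turret controller that explodes on impact and destroys itself.
; On begin play, it points ProjectileMovement at the Projectile component, because that scaled-down mesh is not the root.
; On hit, the server multicasts the explosion at the projectile's location, while clients spawn the emitter locally.
; Both paths then destroy the actor, with no damage logic in the graph.
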(event OnComponentHit(Projectile)
  (params (HitComponent :type Primitive%20Component%20Object%20Reference) (OtherActor :type Actor%20Object%20Reference) (OtherComp :type Primitive%20Component%20Object%20Reference) (NormalImpulse :type Vector :default "0, 0, 0") (Hit :type Hit%20Result%20Structure%20%28by%20ref%29))
  (bind _projectile (Variables|Default|GetProjectile))
  (bind _returnvalue (Transformation|GetWorldLocation _projectile))
  ;[1 1 1] Make projectile explode on hit
  (if (Networking|IsServer)
    (CallFunction|Explode(multicast) _returnvalue)
    (else
      (Effects|SpawnEmitteratLocation "/Game/AI_Turret_Controller/Particles/Explosion_P.Explosion_P" _returnvalue "0, 0, 0" "2.000000,2.000000,2.000000")
      (Actor|DestroyActor))))

(event Custom|Explode%20%28multicast%29
  (params (Location :type Vector))
  ;[1 1 1] Make projectile explode on hit
  (Effects|SpawnEmitteratLocation "/Game/AI_Turret_Controller/Particles/Explosion_P.Explosion_P" Location "0, 0, 0" "2.000000,2.000000,2.000000")
  (Actor|DestroyActor))

(event EventBeginPlay
  ;[1 1 1] Move projectile, since its mesh was scaled down and not used as the root in this projectile
  (Components|Movement|SetUpdatedComponent (Variables|Default|GetProjectileMovement) (Variables|Default|GetProjectile)))

(fn ConstructionScript)