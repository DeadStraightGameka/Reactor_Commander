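; Continuous laser projectile actor for a turret, showing a beam particle from its parent emitter while firing.
; Begin and end fire events relay through multicasts that store the target and toggle beam visibility and Tick.
; Tick pins the beam to the target component, or with none traces forward to max length and calls ApplyDamage on hits.
; A one-second loop from BeginPlay has the server resend beam status to clients.
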(event Custom|Set%20Status%20Clients
  (params (bNewVisibility :type Boolean) (bEnabled :type Boolean))
  ;[1 1 1] Update beam status on start from server
  (Rendering|SetVisibility (Variables|Default|GetP_Beam_Laser) bNewVisibility false)
  (Actor|Tick|SetActorTickEnabled bEnabled))

(event Custom|Begin%20Fire%20%28multicast%29
  (params (Target :type Actor%20Object%20Reference) (InputPin :type Scene%20Component%20Object%20Reference))
  ;[1 1 1] Get Information On When To Or Not Too Fire
  (Variables|Default|SetTarget Target)
  (Variables|Default|SetTarget_Component InputPin)
  (Variables|Default|SetFiring true)
  (Actor|Tick|SetActorTickEnabled true)
  (Rendering|SetVisibility (Variables|Default|GetP_Beam_Laser) true false))

(event Custom|End%20Fire%20Multicast
  (params (Target :type Actor%20Object%20Reference) (InputPin :type Scene%20Component%20Object%20Reference))
  ;[1 1 1] Get Information On When To Or Not Too Fire
  (Variables|Default|SetTarget Target)
  (Variables|Default|SetTarget_Component InputPin)
  (Variables|Default|SetFiring false)
  (Actor|Tick|SetActorTickEnabled false)
  (Rendering|SetVisibility (Variables|Default|GetP_Beam_Laser) false false))

(event EventContinuousLaserSpawn
  (params (Parent%20Controller :type AI%20Turret%20Controller%20BP%20Object%20Reference) (Parent%20Emitter :type Scene%20Component%20Object%20Reference))
  (Variables|Default|SetParent%20Emitter Parent%20Emitter))

(event EventTick
  (params (DeltaSeconds :type Float%20%28single-precision%29))
  (bind _parent_emitter (Variables|Default|GetParent%20Emitter))
  (bind _parent_emitter_2 (Variables|Default|GetParent%20Emitter))
  (bind _returnvalue (Transformation|GetWorldLocation _parent_emitter))
  ;[1 1 1] When Firing, Point Beam At Targets Location. You'd Want To Apply Damage After Here Too Normally.
  (if (Variables|Default|GetFiring)
    (if (== (Variables|Default|GetTarget_Component) 0)
      ;[1 1 1] Get location X distance in front of emitter and trace to it from emitter
      (bind (_outhit _returnvalue_2) (Collision|LineTraceByChannel _returnvalue (+ _returnvalue (* (Math|Vector|GetForwardVector _parent_emitter) (Variables|Default|GetLaser%20Max%20Length))) "TraceTypeQuery1" false (Utilities|Array|MakeArray (Actor|GetParentActor)) "None"))
      ;[1 1 1] Fire at hit location, or end point if no hit found
      (if _returnvalue_2
        (Class|ParticleSystemComponent|SetBeamSourcePoint (Variables|Default|GetP_Beam_Laser) 0 (Transformation|GetWorldLocation (Variables|Default|GetParent%20Emitter)))
        (Class|ParticleSystemComponent|SetBeamEndPoint (Variables|Default|GetP_Beam_Laser) 0 (.location _outhit))
        (Game|Damage|ApplyDamage (.hitactor _outhit) 0.0 0 0)
        (else
          (Class|ParticleSystemComponent|SetBeamSourcePoint (Variables|Default|GetP_Beam_Laser) 0 (Transformation|GetWorldLocation (Variables|Default|GetParent%20Emitter)))
          (Class|ParticleSystemComponent|SetBeamEndPoint (Variables|Default|GetP_Beam_Laser) 0 (+ (Transformation|GetWorldLocation _parent_emitter_2) (* (Math|Vector|GetForwardVector _parent_emitter_2) (Variables|Default|GetLaser%20Max%20Length))))))
      (else
        (Class|ParticleSystemComponent|SetBeamSourcePoint (Variables|Default|GetP_Beam_Laser) 0 (Transformation|GetWorldLocation (Variables|Default|GetParent%20Emitter)))
        (Class|ParticleSystemComponent|SetBeamEndPoint (Variables|Default|GetP_Beam_Laser) 0 (Transformation|GetWorldLocation (Variables|Default|GetTarget_Component)))))))

(event EventBeginPlay
  ;[1 1 1] Update beam status on start from server
  (Utilities|FlowControl|Delay 1.0 :!label _label)
  (Utilities|FlowControl|Sequence
    (:then_0
      (if (Networking|IsServer)
        (CallFunction|SetStatusClients (Variables|/Script/Engine.SceneComponent|GetbVisible (Variables|Default|GetP_Beam_Laser)) (Class|Actor|IsActorTickEnabled))))
    (:then_1
      (goto _label))))

(event EventContinuousLaserBeginFire
  (params (Firing%20At :type Actor%20Object%20Reference) (Firing%20At%20Component :type Scene%20Component%20Object%20Reference) (Aiming%20At%20Location :type Vector :default "0, 0, 0") (Current%20Ammo :type Integer) (Damage%20Multiplier :type Float%20%28single-precision%29) (Forced%20Fire :type Boolean))
  ;[1 1 1] Get Information On When To Or Not Too Fire
  (CallFunction|BeginFire(multicast) Firing%20At Firing%20At%20Component))

(event EventContinuousLaserEndFire
  (params (Firing%20At :type Actor%20Object%20Reference) (Firing%20At%20Component :type Scene%20Component%20Object%20Reference) (Aiming%20At%20Location :type Vector :default "0, 0, 0") (Current%20Ammo :type Integer) (Damage%20Multiplier :type Float%20%28single-precision%29))
  ;[1 1 1] Get Information On When To Or Not Too Fire
  (CallFunction|EndFireMulticast Firing%20At Firing%20At%20Component))

(fn ConstructionScript)