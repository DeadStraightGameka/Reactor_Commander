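; Demo target actor for the AI turret controller that moves two cubes up and down in alternating motion.
; On BeginPlay, the authority runs a timeline that sets each cube's relative Z, scaled by a distance multiplier.
; The second cube mirrors the first by using the absolute offset of the track value from 10.
; When the timeline finishes, it switches direction to loop back and forth.
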(event EventBeginPlay
  (Networking|SwitchHasAuthority
    (:Authority
      ;[1 1 1] Move A Target Up And Down Over Time
      (bind (_direction _track1) (Timeline|Test%20Target Play)
        (:Update
          (Transformation|SetRelativeLocation (Variables|Default|GetTarget_Cube) (Math|Vector|MakeVector 0.0 0.0 (* _track1 (Variables|Default|GetDistance%20Multiplier))) false false)
          (Transformation|SetRelativeLocation (Variables|Default|GetTarget_Cube2) (Math|Vector|MakeVector 0.0 0.0 (* (Math|Float|Absolute(Float) (- _track1 1e+01)) (Variables|Default|GetDistance%20Multiplier))) false false))
        (:Finished
          (if (Utilities|Enum|Equal(Enum) _direction "Forward")
            (Timeline|Test%20Target Reverse)
            (else
              (Timeline|Test%20Target Play))))))))

(fn ConstructionScript)