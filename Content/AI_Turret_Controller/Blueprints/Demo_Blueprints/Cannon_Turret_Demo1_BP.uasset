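; Demo cannon turret Blueprint with two AI turret controllers, one for the main turret and one for a secondary optics turret.
; Acquiring a target enables actor tick, which copies the main controller's target to the optics controller and disables itself when the target check finds none.
; The construction script adds the optics components to the main controller's ignore list, letting it spot enemies through them without ignoring the whole actor.
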(event EventTick
  (params (DeltaSeconds :type Float%20%28single-precision%29))
  ;[1 1 1] Pass On Found Target To Optics Turret Controller So It Points At Same Target, If No Target Then Clear And Disable Ticks
  (if (== 0 (Variables|/Game/AI_Turret_Controller/Blueprints/AI_Turret_Controller_BP/AI_Turret_Controller_BP.AI_Turret_Controller_BP_C|GetTurret%20Target (Variables|Default|GetAI_Turret_Controller%20%28Main%20turret%29)))
    (Actor|Tick|SetActorTickEnabled false)
    (else
      (Variables|/Game/AI_Turret_Controller/Blueprints/AI_Turret_Controller_BP/AI_Turret_Controller_BP.AI_Turret_Controller_BP_C|SetTurret%20Target (Variables|Default|GetAI_Turret_Controller%20%28Optics%29) (Variables|/Game/AI_Turret_Controller/Blueprints/AI_Turret_Controller_BP/AI_Turret_Controller_BP.AI_Turret_Controller_BP_C|GetTurret%20Target (Variables|Default|GetAI_Turret_Controller%20%28Main%20turret%29))))))

(event EventTargetAcquired
  (params (Found%20Target :type Actor%20Object%20Reference) (Parent%20Controller :type AI%20Turret%20Controller%20BP%20Object%20Reference))
  ;[1 1 1] When A Target Is Found Start Tick Events
  (Actor|Tick|SetActorTickEnabled true))

(fn ConstructionScript
  (bind _ai_turret_controller__main_turret_ (Variables|Default|GetAI_Turret_Controller%20%28Main%20turret%29))
  (bind _components_to_ignore (Variables|/Game/AI_Turret_Controller/Blueprints/AI_Turret_Controller_BP/AI_Turret_Controller_BP.AI_Turret_Controller_BP_C|GetComponents%20To%20Ignore _ai_turret_controller__main_turret_))
  ;[1 1 1] Add Optics Turret Components To Ignore List So Main Turret Can Spot Enemies Through Them. If Ignore Self Was Enabled This Woudn't Be Needed, But Its Good To Know How To Do This If You Dont Want Your Turret To Spot Targets Through All Parts Of The Actor (Like A Battleship Cannon Seeing Enemis Through The Command Tower)
  (Utilities|Array|Add _components_to_ignore (Variables|Default|GetOptic_Base2))
  (Utilities|Array|Add _components_to_ignore (Variables|Default|GetOptic_Turret2))
  (Utilities|Array|Add _components_to_ignore (Variables|Default|GetOptic_Barrel2)))