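; Airdrop actor that spawns a single MediumMech_BP with its default controller at its own transform after a randomized delay.
; Tick accumulates delta seconds and compares them against a random threshold of a few seconds, which is rerolled every frame rather than chosen once.
; A Dropped flag stops the timer and prevents further spawns once the mech is out.
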(event EventBeginPlay)

(event Collision|EventActorBeginOverlap
  (params (OtherActor :type Actor%20Object%20Reference)))

(event EventTick
  (params (DeltaSeconds :type Float%20%28single-precision%29))
  ;[1 1 1] Drop Airdrop
  (if (not (Variables|Default|GetDropped))
    (Variables|Default|SetrandomNum (Math|Random|RandomFloatinRange 4.0 14.0))
    (bind _output_get (Variables|Default|SetDelta (+ (Variables|Default|GetDelta) (Utilities|Time|GetWorldDeltaSeconds))))
    (if (>= _output_get (Variables|Default|GetrandomNum))
      (bind _returnvalue (Game|SpawnActorfromClass "/Game/CurrMech_Blueprint/Medium_Mech/MediumMech_BP.MediumMech_BP_C" (Transformation|GetActorTransform self) "Undefined" 0 0))
      (Pawn|SpawnDefaultController _returnvalue)
      (Variables|Default|SetDropped true))))

(fn ConstructionScript)