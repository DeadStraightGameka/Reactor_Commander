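; HUD Blueprint that draws a mech scope aiming reticle at the center of the screen.
; BeginPlay creates a dynamic material instance of the Mech_Scope material and stores it as ScopeAim.
; Each DrawHUD call pushes the ScopeOpacity variable into the material parameter of the same name, then draws the material as a fixed-size square centered on screen.
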(event EventBeginPlay
  (bind _returnvalue (Rendering|Material|CreateDynamicMaterialInstance "/Game/HP_Test_Folder/Blueprints/UI/Mech_Scope.Mech_Scope" :!class /Script/Engine.KismetMaterialLibrary))
  (Variables|Default|SetScope_Aim _returnvalue))

(event EventDrawHUD
  (params (SizeX :type Integer) (SizeY :type Integer))
  (Rendering|Material|SetScalarParameterValue (Variables|Default|GetScope_Aim) "ScopeOpacity" (Variables|Default|GetScope_Opacity) :!class /Script/Engine.MaterialInstanceDynamic)
  (Canvas|DrawMaterial (Variables|Default|GetScope_Aim) (- (* SizeX 0.5) 1.8e+02) (- (* SizeY 0.5) 1.8e+02) 3.6e+02 3.6e+02 1.0 1.0 1.0 1.0))

(fn ConstructionScript)