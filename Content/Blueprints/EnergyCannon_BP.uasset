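; EnergyCannon_BP is a weapon Blueprint for an energy cannon that loads its stats from data.
; On BeginPlay it calls the parent, then reads the "BalisticGun" row of the WeaponSlot data table, despite the cannon's energy name.
; When the row is found, it sets damage, bullet range and rate of fire, then prints them in red.
; It adds no firing logic; overlap and tick events are disabled.
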(event EventBeginPlay
  (|CallParentFunction)
  (bind _returnvalue (Utilities|GetDataTableRow "/Game/JImmy_Test/WeaponSlot.WeaponSlot" "BalisticGun")
    (:then
      (bind _output_get (Variables|Default|SetDamage (.Damage (Utilities|Struct|BreakWeaponStat _returnvalue))))
      (bind _output_get_2 (Variables|Default|SetMaxBulletDistance (.MaxBulletDistance (Utilities|Struct|BreakWeaponStat _returnvalue))))
      (bind _output_get_3 (Variables|Default|SetRateofFire (.RateofFire (Utilities|Struct|BreakWeaponStat _returnvalue))))
      (Development|PrintString (Utilities|String|Append "Damage: " (Utilities|String|ToString(Float) _output_get) "MaxDistance: " (Utilities|String|ToString(Float) _output_get_2) "RateOfFire: " (Utilities|String|ToString(Float) _output_get_3)) true true "(R=1.000000,G=0.000000,B=0.000000,A=1.000000)"))))

(event Collision|EventActorBeginOverlap
  (params (OtherActor :type Actor%20Object%20Reference))
  (|CallParentFunction OtherActor) ; This node is disabled and will not be called.\nDrag off pins to build functionality.
)

(event EventTick
  (params (DeltaSeconds :type Float%20%28single-precision%29))
  (|CallParentFunction DeltaSeconds) ; This node is disabled and will not be called.\nDrag off pins to build functionality.
)

(fn ConstructionScript
  (|CallParentFunction))