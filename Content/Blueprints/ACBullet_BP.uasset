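; Bullet projectile actor that resolves its impact on buildings, destructibles and other objects in its Hit event.
; BuildingConstructor and DestructibleActor targets take fixed radius damage with an explosion effect, and buildings also report a damage event and play a crash sound.
; Other hits push simulating bodies and spawn sparks, while mesh hits apply point damage looked up by weapon name in the WeaponSlot data table, then ricochet audio and self-destruction.
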(event EventBeginPlay)

(event Collision|EventActorBeginOverlap
  (params (OtherActor :type Actor%20Object%20Reference)))

(event Collision|EventHit
  (params (MyComp :type Primitive%20Component%20Object%20Reference) (Other :type Actor%20Object%20Reference) (OtherComp :type Primitive%20Component%20Object%20Reference) (bSelfMoved :type Boolean) (HitLocation :type Vector :default "0, 0, 0") (HitNormal :type Vector :default "0, 0, 0") (NormalImpulse :type Vector :default "0, 0, 0") (Hit :type Hit%20Result%20Structure%20%28by%20ref%29))
  (bind _returnvalue (Transformation|GetActorLocation))
  (Variables|Default|SetSetHitNormal HitNormal)
  (Variables|Default|SetSetHitLocation HitLocation)
  (Utilities|FlowControl|Sequence
    (:then_0
      ;[0.637 0.7857 1] Detect-BuildingConstructor "You may adjust this later if needed".
      (bind _asbuilding_constructor (Utilities|Casting|CastToBuildingConstructor Other))
      (Class|DestructibleComponent|GetDestructibleMesh (Variables|/Script/ApexDestruction.DestructibleActor|GetDestructibleComponent (stale _asdestructible_actor)))
      (Class|DestructibleComponent|ApplyRadiusDamage (Variables|/Game/Blueprints/BuildingConstructor.BuildingConstructor_C|GetMain%20Mesh _asbuilding_constructor) 5e+01 (Variables|Default|GetSetHitLocation) 2e+01 2e+01 true)
      (Class|AISenseDamage|ReportDamageEvent _asbuilding_constructor _asbuilding_constructor (Math|Conversions|ToFloat(Integer) (Variables|Default|GetDamageValue)) (Variables|Default|GetSetHitLocation))
      (Effects|SpawnEmitteratLocation "/Game/Particle_Effect/Particle_explosion_big/Particle_building_explosion.Particle_building_explosion" (Variables|Default|GetSetHitLocation))
      (Audio|PlaySoundatLocation "/Game/SFX_and_BGM/heavy_rock_ruble_pile_impact_or_crash.heavy_rock_ruble_pile_impact_or_crash" (Variables|Default|GetSetHitLocation) "0, 0, 0" 3.0 0.4)
      (Actor|DestroyActor))
    (:then_1
      ;[1 1 1] Detect Destructible objects only
      (bind _asdestructible_actor (Utilities|Casting|CastToDestructibleActor Other)
        (:then
          (Class|DestructibleComponent|ApplyRadiusDamage (Variables|/Script/ApexDestruction.DestructibleActor|GetDestructibleComponent _asdestructible_actor) 2e+01 (Variables|Default|GetSetHitLocation) 5e+01 5e+01 false)
          (Effects|SpawnEmitteratLocation "/Game/Particle_Effect/Particle_explosion_big/Particle_building_explosion.Particle_building_explosion" (Variables|Default|GetSetHitLocation))
          (Actor|DestroyActor))
        (:CastFailed
          (if (Physics|IsSimulatingPhysics OtherComp "None")
            (Physics|AddImpulseatLocation OtherComp (* (Transformation|GetVelocity) 1e+02) _returnvalue "None"))
          (Effects|SpawnEmitteratLocation "/Game/Particle_Effect/Particle_normal_bullet/Particle_normal_bullet_spark.Particle_normal_bullet_spark" (Variables|Default|GetSetHitLocation))
          (bind _asmesh_component (Utilities|Casting|CastToMeshComponent (.HitComponent (Collision|BreakHitResult Hit))))
          (bind _returnvalue_2 (Utilities|GetDataTableRow "/Game/JImmy_Test/WeaponSlot.WeaponSlot" (Variables|Default|GetWeaponName))
            (:then
              (bind _output_get (Variables|Default|SetDamageValue (Math|Float|Truncate (.Damage (Utilities|Struct|BreakWeaponStat _returnvalue_2)))))
              (Game|Damage|ApplyPointDamage (Components|GetOwner _asmesh_component) (Math|Conversions|ToFloat(Integer) _output_get) (Variables|Default|GetSetHitNormal) Hit 0 self)
              (Audio|SpawnSoundatLocation "/Game/SFX_and_BGM/Weapon/HittingSound/Ricochet.Ricochet" _returnvalue)
              (Actor|DestroyActor))))))))

(event EventTick
  (params (DeltaSeconds :type Float%20%28single-precision%29)))

(fn ConstructionScript
  (|CallParentFunction))