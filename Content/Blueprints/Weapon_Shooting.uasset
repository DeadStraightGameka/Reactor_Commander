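; Weapon logic that fires an autocannon or laser from its owner, using muzzle and particle components found by name.
; Server events relay to multicasts that read WeaponSlot data table rows for cooldown and heat added to the target.
; The autocannon spawns projectiles and decrements ammo, gated by a DoOnce reload.
; The laser fires repeated line-trace shots through a DoN limit, drawing beam particles and applying point damage, including to destructibles and buildings.
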(event Custom|RunOnServerAutoCannon
  (params (Target :type Base%20Mech%20BP%20Object%20Reference))
  ;[1 1 1] AutoCannon Shooting Mechanism
  (CallFunction|MulticastAutoCannon Target))

(event Custom|MulticastLaserWeapon
  (params (InputPin :type Base%20Mech%20BP%20Object%20Reference))
  ;[1 1 1] LaserWeapon Shooting Mechanism
  (Utilities|FlowControl|Sequence
    (:then_0
      (bind _returnvalue (Utilities|GetDataTableRow "/Game/JImmy_Test/WeaponSlot.WeaponSlot" "LaserGun")
        (:then
          (if (Variables|WeaponBehavior|GetIsReloadDone)
            (bind _counter (Utilities|FlowControl|DoN 20 :!label _label)
              (:Exit
                (bind _newparam (CallFunction|ShootingLaser))
                (Utilities|FlowControl|Sequence
                  (:then_0
                    (Utilities|FlowControl|Delay (.RateofFire (Utilities|Struct|BreakWeaponStat _returnvalue)))
                    (if (>= _counter 20)
                      (Utilities|FlowControl|Delay (.MaxCooldown (Utilities|Struct|BreakWeaponStat _returnvalue)))
                      (Variables|WeaponBehavior|SetIsReloadDone true)
                      (goto _label Reset)
                      (else
                        (goto _label))))
                  (:then_1
                    (Utilities|FlowControl|Delay 0.1)
                    (Variables|WeaponBehavior|SetIsReloadDone false))
                  (:then_2
                    (Utilities|FlowControl|Delay 0.5)
                    (Effects|Components|ParticleSystem|SetTemplate _newparam 0))
                  (:then_3
                    (Variables|/Game/Blueprints/BaseMech_BP.BaseMech_BP_C|SetHeatGenerate InputPin (+ (Variables|/Game/Blueprints/BaseMech_BP.BaseMech_BP_C|GetHeatGenerate InputPin) (.HeatGenerate (Utilities|Struct|BreakWeaponStat _returnvalue))))))))))))
    (:then_1
      (if (Variables|WeaponBehavior|GetIsReloadDone)
        (Audio|PlaySoundatLocation "/Game/SFX_and_BGM/Weapon/ShootingSound/Laser_Cue.Laser_Cue" "0, 0, 0")))))

(event Custom|MulticastAutoCannon
  (params (Target :type Base%20Mech%20BP%20Object%20Reference))
  ;[1 1 1] AutoCannon Shooting Mechanism
  (bind _returnvalue (Utilities|GetDataTableRow "/Game/JImmy_Test/WeaponSlot.WeaponSlot" (Variables|Default|GetWeaponName))
    (:then
      (if (Variables|WeaponBehavior|GetIsReloadDone)
        (Utilities|FlowControl|DoOnce false :!label _label
          (:Completed
            (Utilities|FlowControl|Sequence
              (:then_0
                (CallFunction|ShootingProjectile)
                (Variables|WeaponBehavior|SetIsReloadDone false)
                (Utilities|FlowControl|Delay 1.0)
                (Audio|PlaySoundatLocation "/Game/SFX_and_BGM/Weapon/ShootingSound/Auto_Cannon_Reload_Cue.Auto_Cannon_Reload_Cue" "0, 0, 0")
                (Utilities|FlowControl|Delay (.MaxCooldown (Utilities|Struct|BreakWeaponStat _returnvalue)))
                (bind _output_get (Variables|WeaponBehavior|SetIsReloadDone true))
                (if (and _output_get (!= (Variables|WeaponBehavior|GetCurrentAmmo) 0))
                  (goto _label Reset)))
              (:then_1
                (Variables|WeaponBehavior|SetCurrentAmmo (- (Variables|WeaponBehavior|GetCurrentAmmo) 1)))
              (:then_2
                (Variables|/Game/Blueprints/BaseMech_BP.BaseMech_BP_C|SetHeatGenerate Target (+ (Variables|/Game/Blueprints/BaseMech_BP.BaseMech_BP_C|GetHeatGenerate Target) (.HeatGenerate (Utilities|Struct|BreakWeaponStat _returnvalue))))))))))))

(event Custom|RunOnServerLaserWeapon
  (params (InputPin :type Base%20Mech%20BP%20Object%20Reference))
  ;[1 1 1] LaserWeapon Shooting Mechanism
  (CallFunction|MulticastLaserWeapon InputPin))

(event EventBeginPlay
  (Utilities|FlowControl|Sequence
    (:then_0
      (if (not (Variables|FindingOwner|GetGameStarted))
        (Variables|FindingOwner|SetOwner (Components|GetOwner))
        (CallFunction|SearchAllActorComponent)
        (Variables|FindingOwner|SetGameStarted true)))
    (:then_1
      (bind _returnvalue (Utilities|GetDataTableRow "/Game/JImmy_Test/WeaponSlot.WeaponSlot" (Variables|Default|GetWeaponName))
        (:then
          (Variables|WeaponBehavior|SetCurrentAmmo (.MaxAmmo (Utilities|Struct|BreakWeaponStat _returnvalue))))))))

(event EventTick
  (params (DeltaSeconds :type Float%20%28single-precision%29)))

(fn ShootingProjectile
  (bind _arrow (Variables|FindingOwner|GetArrow))
  (bind _returnvalue (Transformation|GetWorldTransform _arrow))
  (bind (_location _rotation) (Math|Transform|BreakTransform _returnvalue))
  (Audio|PlaySoundatLocation "/Game/SFX_and_BGM/Weapon/ShootingSound/Auto_Cannon_Cue.Auto_Cannon_Cue" _location)
  (Effects|SpawnEmitteratLocation "/Game/Particle_Effect/Particke_autocannon/Particle_Autocannon_muzzle_flash.Particle_Autocannon_muzzle_flash" _location _rotation "0.500000,0.500000,0.500000")
  (Game|SpawnActorfromClass (Variables|WeaponBehavior|GetProjectile) _returnvalue "AlwaysSpawn" 0 0))

(fn SearchAllActorComponent
  (Utilities|FlowControl|Sequence
    (:then_0
      (bind _output_get (Variables|FindingOwner|SetTargetList1 (Actor|GetComponentsByClass (Variables|FindingOwner|GetOwner) "/Script/Engine.SceneComponent")))
      (for _array_element _output_get
        (if (Utilities|String|Contains (Utilities|GetDisplayName _array_element) (Utilities|String|ToString(Text) (Utilities|Text|FormatText "{A}MuzzleHole{X}" (Variables|FindingOwner|GetComponentName) (Variables|FindingOwner|GetIndexNumber))))
          (Variables|FindingOwner|SetArrow _array_element))))
    (:then_1
      (bind _output_get_2 (Variables|FindingOwner|SetTargetList2 (Actor|GetComponentsByClass (Variables|FindingOwner|GetOwner) "/Script/Engine.ParticleSystemComponent")))
      (for _array_element_2 _output_get_2
        (if (Utilities|String|Contains (Utilities|GetDisplayName _array_element_2) (Utilities|String|ToString(Text) (Utilities|Text|FormatText "{A}ParticleSystem{X}" (Variables|FindingOwner|GetComponentName) (Variables|FindingOwner|GetIndexNumber))))
          (Variables|Default|SetParSysTarget _array_element_2))))))

(fn ShootingLaser
  (bind _arrow (Variables|FindingOwner|GetArrow))
  (bind _returnvalue (Transformation|GetWorldTransform _arrow))
  (bind _returnvalue_2 (Transformation|GetWorldRotation _arrow))
  (bind _location (Math|Transform|BreakTransform _returnvalue))
  (bind _returnvalue_3 (Math|Rotator|GetRotationXVector _returnvalue_2))
  (bind _returnvalue_4 (* _returnvalue_3 1e+05))
  (bind _returnvalue_5 (+ _location _returnvalue_4))
  (bind _asparticle_system_component (Utilities|Casting|CastToParticleSystemComponent (Variables|Default|GetParSysTarget)))
  (Effects|Components|ParticleSystem|SetTemplate _asparticle_system_component (Variables|Default|GetParticleType))
  (Class|ParticleSystemComponent|SetBeamSourcePoint _asparticle_system_component 0 _location)
  (bind (_outhit _returnvalue_6) (Collision|LineTraceForObjects _location _returnvalue_5 (Utilities|Array|MakeArray "ObjectTypeQuery1" "ObjectTypeQuery2" "ObjectTypeQuery3" "ObjectTypeQuery4" "ObjectTypeQuery6") false 0 "None"))
  (if _returnvalue_6
    (bind _returnvalue_7 (Utilities|GetDataTableRow "/Game/JImmy_Test/WeaponSlot.WeaponSlot" "LaserGun")
      (:then
        (if (> (.Distance (Collision|BreakHitResult _outhit)) (.MaxBulletDistance (Utilities|Struct|BreakWeaponStat _returnvalue_7)))
          (Class|ParticleSystemComponent|SetBeamTargetPoint _asparticle_system_component 0 _returnvalue_5 :!label _label)
          (return _asparticle_system_component)
          (else
            (Class|ParticleSystemComponent|SetBeamTargetPoint _asparticle_system_component 0 (.Location (Collision|BreakHitResult _outhit)))
            (Effects|SpawnEmitteratLocation "/Game/Particle_Effect/Particle_laser_spark/Particle_laser_spark.Particle_laser_spark" (.Location (Collision|BreakHitResult _outhit)))
            (Utilities|FlowControl|Sequence
              (:then_0
                (bind _asmesh_component (Utilities|Casting|CastToMeshComponent (.HitComponent (Collision|BreakHitResult _outhit))))
                (bind _returnvalue_8 (Utilities|GetDataTableRow "/Game/JImmy_Test/WeaponSlot.WeaponSlot" "LaserGun")
                  (:then
                    (Game|Damage|ApplyPointDamage (Components|GetOwner _asmesh_component) (.Damage (Utilities|Struct|BreakWeaponStat _returnvalue_8)) (.Location (Collision|BreakHitResult _outhit)) _outhit (Pawn|GetController (Variables|Default|GetOwnedChar))))))
              (:then_1
                (bind _asdestructible_actor (Utilities|Casting|CastToDestructibleActor (.HitActor (Collision|BreakHitResult _outhit))))
                (Game|Damage|ApplyPointDamage _asdestructible_actor 0.02 (.Location (Collision|BreakHitResult _outhit)) _outhit))
              (:then_2
                (bind _asbuilding_constructor (Utilities|Casting|CastToBuildingConstructor (.HitActor (Collision|BreakHitResult _outhit))))
                (Game|Damage|ApplyPointDamage _asbuilding_constructor 0.03 (.Location (Collision|BreakHitResult _outhit)) _outhit))
              (:then_3
                (return _asparticle_system_component)))))))
    (else
      (goto _label))))