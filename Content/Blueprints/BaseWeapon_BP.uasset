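; Base weapon Blueprint with three firing functions for laser, autocannon and rocket shots, all originating from GunMesh1 sockets.
; ShootEnergy draws a beam using a caller-supplied trace result, capped by the WeaponSlot table's LaserGun range.
; In-range hits spawn sparks and apply table damage to mesh owners, or fixed damage to non-mesh destructible or BuildingConstructor hits.
; ShootProjectile and ShootRocket share sound and muzzle flash, spawning ACBullet_BP or Rocket_BP respectively.
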(event EventBeginPlay)

(event Collision|EventActorBeginOverlap
  (params (OtherActor :type Actor%20Object%20Reference)))

(event EventTick
  (params (DeltaSeconds :type Float%20%28single-precision%29)))

(fn ConstructionScript)

(fn ShootEnergy
  (params (StartLocation :type Name) (ReturnValue :type Boolean) (OutHit :type Hit%20Result%20Structure) (EndLocation :type Vector))
  (bind (_bblockinghit _binitialoverlap _time _distance _location _impactpoint _normal _impactnormal _physmat _hitactor _hitcomponent) (Collision|BreakHitResult OutHit))
  (bind _particlesystem (Variables|Default|GetParticleSystem))
  (Effects|Components|ParticleSystem|SetTemplate _particlesystem "/Game/Particle_Effect/Particle_laser_beam/Particle_laserbeam.Particle_laserbeam")
  (Class|ParticleSystemComponent|SetBeamSourcePoint _particlesystem 0 (.Location (Math|Transform|BreakTransform (Transformation|GetSocketTransform (Variables|Default|GetGunMesh1) StartLocation "RTS_World"))))
  (if ReturnValue
    (bind _returnvalue (Utilities|GetDataTableRow "/Game/JImmy_Test/WeaponSlot.WeaponSlot" "LaserGun")
      (:then
        (if (> _distance (.MaxBulletDistance (Utilities|Struct|BreakWeaponStat _returnvalue)))
          (Class|ParticleSystemComponent|SetBeamTargetPoint _particlesystem 0 EndLocation :!label _label)
          (else
            (Class|ParticleSystemComponent|SetBeamTargetPoint _particlesystem 0 _location)
            (Effects|SpawnEmitteratLocation "/Game/Particle_Effect/Particle_laser_spark/Particle_laser_spark.Particle_laser_spark" _location)
            (bind _asmesh_component (Utilities|Casting|CastToMeshComponent _hitcomponent)
              (:then
                (bind _returnvalue_2 (Utilities|GetDataTableRow "/Game/JImmy_Test/WeaponSlot.WeaponSlot" "LaserGun")
                  (:then
                    (Game|Damage|ApplyPointDamage (Components|GetOwner _asmesh_component) (.Damage (Utilities|Struct|BreakWeaponStat _returnvalue_2)) _location OutHit (Pawn|GetController (Variables|Default|GetOwnedChar)) self))))
              (:CastFailed
                (bind _asdestructible_actor (Utilities|Casting|CastToDestructibleActor _hitactor)
                  (:then
                    (Game|Damage|ApplyPointDamage _asdestructible_actor 0.02 _location OutHit))
                  (:CastFailed
                    (bind _asbuilding_constructor (Utilities|Casting|CastToBuildingConstructor _hitactor))
                    (Game|Damage|ApplyPointDamage _asbuilding_constructor 0.03 _location OutHit)))))))))
    (else
      (goto _label))))

(fn ShootProjectile
  (params (WeaponSocket :type Name))
  (bind _gunmesh1 (Variables|Default|GetGunMesh1))
  (bind _returnvalue (Transformation|GetSocketTransform _gunmesh1 WeaponSocket "RTS_World"))
  (bind (_location _rotation) (Math|Transform|BreakTransform _returnvalue))
  (Audio|PlaySoundatLocation "/Game/SFX_and_BGM/Weapon/ShootingSound/Auto_Cannon_Cue.Auto_Cannon_Cue" _location)
  (Effects|SpawnEmitteratLocation "/Game/Particle_Effect/Particke_autocannon/Particle_Autocannon_muzzle_flash.Particle_Autocannon_muzzle_flash" _location _rotation "0.500000,0.500000,0.500000")
  (Game|SpawnActorfromClass "/Game/Blueprints/ACBullet_BP.ACBullet_BP_C" _returnvalue "AlwaysSpawn" 0 0))

(fn ShootRocket
  (params (WeaponSocket :type Name))
  (bind _gunmesh1 (Variables|Default|GetGunMesh1))
  (bind _returnvalue (Transformation|GetSocketTransform _gunmesh1 WeaponSocket "RTS_World"))
  (bind (_location _rotation) (Math|Transform|BreakTransform _returnvalue))
  (Audio|PlaySoundatLocation "/Game/SFX_and_BGM/Weapon/ShootingSound/Auto_Cannon_Cue.Auto_Cannon_Cue" _location)
  (Effects|SpawnEmitteratLocation "/Game/Particle_Effect/Particke_autocannon/Particle_Autocannon_muzzle_flash.Particle_Autocannon_muzzle_flash" _location _rotation "0.500000,0.500000,0.500000")
  (Game|SpawnActorfromClass "/Game/Blueprints/Rocket_BP.Rocket_BP_C" _returnvalue "AlwaysSpawn" 0 0))