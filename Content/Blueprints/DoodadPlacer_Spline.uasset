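; Spline-based doodad placer that scatters copies of a mesh at even spacing along an editable, optionally closed path.
; The construction script divides spline length by ObjectSpacing and adds a scaled static mesh with assigned material, or a destructible mesh, at each step.
; Instances follow the spline's roll and yaw but not pitch, and PathScale sets the actor scale.
; Spline-mesh wire logic is present but disconnected.
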(event EventBeginPlay)

(event Collision|EventActorBeginOverlap
  (params (OtherActor :type Actor%20Object%20Reference)))

(event EventTick
  (params (DeltaSeconds :type Float%20%28single-precision%29)))

(fn ConstructionScript
  (bind _spline (Variables|Default|GetSpline))
  (bind _spline_2 (Variables|Default|GetSpline))
  (bind _object_scale (Variables|MeshTransform|GetObject%20Scale))
  (bind _object_spacing (Variables|MeshTransform|GetObject%20Spacing))
  (Spline|SetClosedLoop _spline (Variables|MeshTransform|GetCloseLoop) true)
  (for _index (range 0 (.ReturnValue (Math|Float|Division(WholeandRemainder) (Spline|GetSplineLength _spline) _object_spacing)))
    (bind _output_get (Variables|Default|SetIndexTracker _index))
    (if (Variables|MeshSettings|GetDestructible)
      (bind _returnvalue (AddComponent|AddDestructibleComponent true (Math|Transform|MakeTransform (Spline|GetLocationatDistanceAlongSpline _spline_2 (* _output_get _object_spacing) "World") (Math|Rotator|MakeRotator (.roll (Spline|GetRotationatDistanceAlongSpline _spline_2 (* _output_get _object_spacing) "World")) 0.0 (.yaw (Spline|GetRotationatDistanceAlongSpline _spline_2 (* _output_get _object_spacing) "World"))) (Math|Vector|MakeVector _object_scale _object_scale _object_scale))))
      (Class|DestructibleComponent|SetDestructibleMesh _returnvalue (Variables|MeshSettings|GetDestructible%20Mesh))
      (else
        ;[1 1 1] AddMeshUndMaterial
        (bind _returnvalue_2 (AddComponent|AddStaticMeshComponent true (Math|Transform|MakeTransform (Spline|GetLocationatDistanceAlongSpline _spline_2 (* _output_get _object_spacing) "World") (Math|Rotator|MakeRotator (.roll (Spline|GetRotationatDistanceAlongSpline _spline_2 (* _output_get _object_spacing) "World")) 0.0 (.yaw (Spline|GetRotationatDistanceAlongSpline _spline_2 (* _output_get _object_spacing) "World"))) (Math|Vector|MakeVector _object_scale _object_scale _object_scale))))
        (Components|StaticMesh|SetStaticMesh _returnvalue_2 (Variables|MeshSettings|GetSelect%20Mesh))
        (Rendering|Material|SetMaterial _returnvalue_2 0 (Variables|MeshSettings|GetAssign%20Material))))
    ;[1 1 1] SplineScale
    (Transformation|SetActorScale3D (Variables|MeshTransform|GetPathScale))))