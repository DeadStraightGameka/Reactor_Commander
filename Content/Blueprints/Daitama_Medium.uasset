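; Player-controlled medium Daitama mech that toggles between first and third person, fires its first two weapons on input, and halves movement once a leg is destroyed.
; Each tick, a camera trace rotates up to two ballistic and two laser weapons toward the aim point, clamped to WeaponSlot table ranges.
; The tick also runs heat logic: timer-driven cooldown, overheat with hysteresis that stops running, animation updates and a high-heat sound.
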(event EventBeginPlay)

(event Collision|EventActorBeginOverlap
  (params (OtherActor :type Actor%20Object%20Reference)))

(event EventTick
  (params (DeltaSeconds :type Float%20%28single-precision%29))
  (bind _charactermovement (Variables|Character|GetCharacterMovement))
  (CallFunction|ParentTick)
  (Utilities|FlowControl|Sequence
    (:then_0
      (Utilities|AimSystem))
    (:then_1
      (Utilities|HeatSystem))
    (:then_2
      (if (Variables|Default|GetIsOneLegDestroyed)
        (Utilities|FlowControl|DoOnce false
          (:Completed
            (Variables|/Script/Engine.CharacterMovementComponent|SetMaxAcceleration _charactermovement (/ (Variables|/Script/Engine.CharacterMovementComponent|GetMaxAcceleration _charactermovement) 2.0))
            (Variables|/Script/Engine.CharacterMovementComponent|SetMaxWalkSpeed _charactermovement (/ (Variables|/Script/Engine.CharacterMovementComponent|GetMaxWalkSpeed _charactermovement) 2.0))))))))

(event Input|ActionEvents|InputActionSwitchCamera
  (params (Key :type Key%20Structure))
  (:Pressed
    (CallFunction|SwitchCameraFunction)))

(event Input|ActionEvents|InputActionFireCurrentWeapon
  (params (Key :type Key%20Structure))
  (:Pressed
    (Default|ShootingProjectile1 (Variables|/Game/Blueprints/BaseWeapon_BP.BaseWeapon_BP_C|GetWeapon_Shooting (Variables|Default|GetEquippedWeapon01)))))

(fn ConstructionScript
  (|CallParentFunction))

(fn SwitchCameraFunction
  (bind _springarm_0 (Variables|Default|GetSpringArm_0))
  (if (Variables|Default|GetSwitchCamera)
    (Variables|/Script/Engine.SpringArmComponent|SetTargetArmLength _springarm_0 0.0)
    (Variables|/Script/Engine.SpringArmComponent|SetTargetOffset _springarm_0 "0, 0, 0")
    (Class|PrimitiveComponent|SetOwnerNoSee (Variables|Default|GetFrontTorso) true)
    (Variables|Default|SetSwitchCamera false)
    (else
      (Variables|/Script/Engine.SpringArmComponent|SetTargetArmLength _springarm_0 1.5e+03)
      (Variables|/Script/Engine.SpringArmComponent|SetTargetOffset _springarm_0 "0, 0,360.000000")
      (Class|PrimitiveComponent|SetOwnerNoSee (Variables|Default|GetFrontTorso) false)
      (Variables|Default|SetSwitchCamera true))))