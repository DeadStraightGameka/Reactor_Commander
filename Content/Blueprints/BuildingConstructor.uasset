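; BuildingConstructor procedurally builds a modular wall or building grid in its Construction Script, with no active runtime logic.
; Nested Floors and Segments loops add either destructible or static mesh components, chosen by UseDestructibleMesh.
; Each piece is offset in X and Z by the mesh's bounds extent times a spacing multiplier.
; Both branches share a Material or MaterialInstance step, which targets the static mesh component.
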(event EventBeginPlay)

(event Collision|EventActorBeginOverlap
  (params (OtherActor :type Actor%20Object%20Reference)))

(event EventTick
  (params (DeltaSeconds :type Float%20%28single-precision%29)))

(fn ConstructionScript
  (bind _static_mesh (Variables|SetMesh|GetStatic%20Mesh))
  (bind _returnvalue (StaticMesh|GetBounds _static_mesh))
  (bind _boxextent (Math|BoxSphereBounds|BreakBoxSphereBounds _returnvalue))
  (bind (_x _y _z) (Math|Vector|BreakVector _boxextent))
  ;[1 1 1] ComponentTypeConditionCheck
  (if (Variables|SetMesh|GetUse%20Destructible%20Mesh?)
    ;[1 1 1] DestructibleMesh
    (for _index (range 0 (- (Variables|MeshProperties|GetFloors) 1))
      ;;[1 1 1] GetTargetScale
      (bind _returnvalue_2 (StaticMesh|GetBounds (Variables|SetMesh|GetDestructible%20Mesh)))
      (for _index_2 (range 0 (- (Variables|MeshProperties|GetSegments) 1))
        (bind _returnvalue_3 (AddComponent|AddDestructibleComponent false (Math|Transform|MakeTransform (Math|Vector|MakeVector (* (* _index_2 (.X (Math|Vector|BreakVector (.BoxExtent (Math|BoxSphereBounds|BreakBoxSphereBounds _returnvalue_2))))) (Variables|MeshProperties|GetHorizontal%20Spacing)) 0.0 (* (* _index (.Z (Math|Vector|BreakVector (.BoxExtent (Math|BoxSphereBounds|BreakBoxSphereBounds _returnvalue_2))))) (Variables|MeshProperties|GetVertical%20Spacing))))))
        (Class|DestructibleComponent|SetDestructibleMesh _returnvalue_3 (Variables|SetMesh|GetDestructible%20Mesh))
        ;[1 1 1] StaticMesh
        (if (Variables|Material|GetUse%20Material%20Instance?)
          (Rendering|Material|SetMaterial (stale _returnvalue_4) 0 (Variables|Material|GetMaterial%20Instance))
          (else
            (Rendering|Material|SetMaterial (stale _returnvalue_4) 0 (Variables|Material|GetMaterial))))))
    (else
      (for _index_3 (range 0 (- (Variables|MeshProperties|GetFloors) 1))
        (for _index_4 (range 0 (- (Variables|MeshProperties|GetSegments) 1))
          (bind _returnvalue_4 (AddComponent|AddStaticMeshComponent false (Math|Transform|MakeTransform (Math|Vector|MakeVector (* (* _index_4 _x) (Variables|MeshProperties|GetHorizontal%20Spacing)) 0.0 (* (* _index_3 _z) (Variables|MeshProperties|GetVertical%20Spacing))))))
          (Components|StaticMesh|SetStaticMesh _returnvalue_4 (Variables|SetMesh|GetStatic%20Mesh))
          (if (Variables|Material|GetUse%20Material%20Instance?)
            (Rendering|Material|SetMaterial _returnvalue_4 0 (Variables|Material|GetMaterial%20Instance))
            (else
              (Rendering|Material|SetMaterial _returnvalue_4 0 (Variables|Material|GetMaterial)))))))))