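; Projectile actor that deals damage, effects and sound on impact, with its owning pawn set through SetOwnedPawn.
; BuildingConstructor hits get radial falloff damage, while DestructibleActor hits get radius damage with impulse, both with explosion particles.
; Other hits push physics bodies and spark, then mesh hits apply point damage from the WeaponSlot table's BalisticGun row, credited to the owner's controller.
; These damaging paths destroy the projectile.
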(event Custom|SetOwnedPawn
  (params (OwningPawn :type Current%20Mech%20Object%20Reference))
  (bind _output_get (Variables|Default|SetOwnedChar OwningPawn))
  (Actor|SetOwner _output_get))

(event Collision|EventActorBeginOverlap
  (params (OtherActor :type Actor%20Object%20Reference))
  (|CallParentFunction OtherActor) ; This node is disabled and will not be called.\nDrag off pins to build functionality.
)

(event Collision|EventHit
  (params (MyComp :type Primitive%20Component%20Object%20Reference) (Other :type Actor%20Object%20Reference) (OtherComp :type Primitive%20Component%20Object%20Reference) (bSelfMoved :type Boolean) (HitLocation :type Vector :default "0, 0, 0") (HitNormal :type Vector :default "0, 0, 0") (NormalImpulse :type Vector :default "0, 0, 0") (Hit :type Hit%20Result%20Structure%20%28by%20ref%29))
  (bind (_bblockinghit _binitialoverlap _time _distance _location _impactpoint _normal _impactnormal _physmat _hitactor _hitcomponent _hitbonename _hititem _faceindex _tracestart) (Collision|BreakHitResult Hit))
  (bind _returnvalue (Transformation|GetActorLocation))
  (Utilities|FlowControl|Sequence
    (:then_0
      ;[1 1 1] Detect-BuildingConstructor "You may adjust this later if needed".
      (Utilities|Casting|CastToBuildingConstructor Other)
      (Class|GameplayStatics|ApplyRadialDamagewithFalloff 3e+01 1e+01 HitLocation 4e+01 7e+01 1e+02 0 0 0 0 "ECC_Visibility")
      (Effects|SpawnEmitteratLocation "/Game/Particle_Effect/Particle_explosion_big/Particle_building_explosion.Particle_building_explosion" HitLocation)
      (Audio|PlaySoundatLocation "/Game/SFX_and_BGM/heavy_rock_ruble_pile_impact_or_crash.heavy_rock_ruble_pile_impact_or_crash" HitLocation "0, 0, 0" 3.0 0.4)
      (Actor|DestroyActor))
    (:then_1
      (bind _asdestructible_actor (Utilities|Casting|CastToDestructibleActor Other)
        (:then
          (Class|DestructibleComponent|ApplyRadiusDamage (Variables|/Script/ApexDestruction.DestructibleActor|GetDestructibleComponent _asdestructible_actor) 2e+01 HitLocation 5e+01 5e+01 false)
          (Effects|SpawnEmitteratLocation "/Game/Particle_Effect/Particle_explosion_big/Particle_building_explosion.Particle_building_explosion" HitLocation))
        (:CastFailed
          (if (Physics|IsSimulatingPhysics OtherComp "None")
            (Physics|AddImpulseatLocation OtherComp (* (Transformation|GetVelocity) 1e+02) _returnvalue "None"))
          (Effects|SpawnEmitteratLocation "/Game/Particle_Effect/Particle_normal_bullet/Particle_normal_bullet_spark.Particle_normal_bullet_spark" HitLocation)
          (bind _asmesh_component (Utilities|Casting|CastToMeshComponent _hitcomponent))
          (bind _returnvalue_2 (Utilities|GetDataTableRow "/Game/JImmy_Test/WeaponSlot.WeaponSlot" "BalisticGun")
            (:then
              (Game|Damage|ApplyPointDamage (Components|GetOwner _asmesh_component) (.Damage (Utilities|Struct|BreakWeaponStat _returnvalue_2)) _tracestart Hit (Pawn|GetController (Variables|Default|GetOwnedChar)) self)
              (Audio|SpawnSoundatLocation "/Game/SFX_and_BGM/Weapon/HittingSound/Ricochet.Ricochet" _returnvalue)))))
      (Actor|DestroyActor))))

(event EventTick
  (params (DeltaSeconds :type Float%20%28single-precision%29))
  (|CallParentFunction DeltaSeconds) ; This node is disabled and will not be called.\nDrag off pins to build functionality.
)

(fn ConstructionScript
  (|CallParentFunction))