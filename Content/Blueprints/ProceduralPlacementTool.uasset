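; Procedural placement actor that lays copies of a chosen static mesh along an editable spline.
; Its Construction Script steps along the spline length at a set spacing, adding scaled mesh components with the assigned material and the spline's yaw and roll.
; It also applies the loop setting and actor-wide path scale.
; The Wire flag suppresses mesh placement; the spline-mesh wire logic is unconnected, and the Event Graph is empty.
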(event EventBeginPlay)

(event Collision|EventActorBeginOverlap
  (params (OtherActor :type Actor%20Object%20Reference)))

(event EventTick
  (params (DeltaSeconds :type Float%20%28single-precision%29)))

(fn ConstructionScript
  (bind _spline (Variables|Default|GetSpline))
  (bind _object_scale (Variables|Default|GetObject%20Scale))
  (bind _object_spacing (Variables|Default|GetObject%20Spacing))
  (for _index (range 0 (.ReturnValue (Math|Float|Division(WholeandRemainder) (Spline|GetSplineLength (Variables|Default|GetSpline)) _object_spacing)))
    (bind _output_get (Variables|Default|SetIndexTracker _index))
    (Spline|SetClosedLoop _spline (Variables|Default|GetCloseLoop) true)
    (if (not (Variables|Default|GetWire))
      ;[1 1 1] AddMeshUndMaterial
      (bind _returnvalue (AddComponent|AddStaticMeshComponent true (Math|Transform|MakeTransform (Spline|GetLocationatDistanceAlongSpline _spline (* _output_get _object_spacing) "World") (Math|Rotator|MakeRotator (.roll (Spline|GetRotationatDistanceAlongSpline _spline (* _output_get _object_spacing) "World")) 0.0 (.yaw (Spline|GetRotationatDistanceAlongSpline _spline (* _output_get _object_spacing) "World"))) (Math|Vector|MakeVector _object_scale _object_scale _object_scale))))
      (Components|StaticMesh|SetStaticMesh _returnvalue (Variables|Default|GetSelect%20Mesh))
      (Rendering|Material|SetMaterial _returnvalue 0 (Variables|Default|GetAssign%20Material))
      ;[1 1 1] SplineScale
      (Transformation|SetActorScale3D (Variables|Default|GetPathScale)))))