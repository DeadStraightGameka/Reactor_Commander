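; Track generator Blueprint that builds a road with optional guard rails along a spline in its Construction Script.
; It resizes a per-point data array to match the spline, padding with defaults.
; Each segment gets spline mesh components with bank, width and thickness set from both endpoints, optional collision, and per-point rail toggles.
; The track can close into a loop, and a debug flag labels spline points with their index.
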(event EventBeginPlay)

(event Collision|EventActorBeginOverlap
  (params (OtherActor :type Actor%20Object%20Reference)))

(event EventTick
  (params (DeltaSeconds :type Float%20%28single-precision%29)))

(fn ConstructionScript
  (bind _roaddataarray (Variables|Default|GetRoadDataArray))
  (bind _currentloopindex (Variables|Default|GetCurrentLoopIndex))
  (bind _output (Utilities|Array|Get(acopy) _roaddataarray _currentloopindex))
  (Utilities|FlowControl|Sequence
    (:then_0
      (|SplinePointsCount))
    (:then_1
      (|BuildRoadData))
    (:then_2
      (|ConstructionLoop)
      (Variables|Default|SetDrawLeftGuardRail (.leftguardrail _output))
      (Variables|Default|SetDrawRightGuardRail (.rightguardrail _output))
      (Utilities|FlowControl|Sequence
        (:then_0
          ;[1 1 1] Create_RoadMesh
          (CallFunction|BuildTrackElements (Variables|Default|GetCurrentLoopIndex) (Variables|Default|GetRoadMesh)))
        (:then_1
          ;[1 1 1] Create_LeftGuardRail
          (if (Variables|Default|GetDrawLeftGuardRail)
            (CallFunction|BuildTrackElements (Variables|Default|GetCurrentLoopIndex) (Variables|Default|GetLeftGuardRailMesh))))
        (:then_2
          ;[1 1 1] Create_RightGuardRail
          (if (Variables|Default|GetDrawRightGuardRail)
            (CallFunction|BuildTrackElements (Variables|Default|GetCurrentLoopIndex) (Variables|Default|GetRightGuardRailMesh))))))
    (:then_3
      (|ShowSplineNumber))))

(fn BuildTrackElements
  (params (LoopIndex :type Integer) (TrackElementsMesh :type Static%20Mesh%20Object%20Reference))
  (LocalVariables|SetLocal_CurrentLoopIndex LoopIndex)
  (LocalVariables|SetLocal_NextLoopIndex (Math|Integer|%(Integer) (+ LoopIndex 1) (Variables|Default|GetNumberOfSplinePoints)))
  (LocalVariables|SetLocal_TrackElements TrackElementsMesh)
  (Utilities|FlowControl|Sequence
    (:then_0
      ;[1 1 1] Set_VertexPointsForSplines
      (LocalVariables|SetLocal_StartLocation (.Location (Spline|GetLocationandTangentatSplinePoint (Variables|Default|GetRoadSpline) (LocalVariables|GetLocal_CurrentLoopIndex) "Local")))
      (LocalVariables|SetLocal_StartTangent (.Tangent (Spline|GetLocationandTangentatSplinePoint (Variables|Default|GetRoadSpline) (LocalVariables|GetLocal_CurrentLoopIndex) "Local")))
      (LocalVariables|SetLocal_EndLocation (.Location (Spline|GetLocationandTangentatSplinePoint (Variables|Default|GetRoadSpline) (LocalVariables|GetLocal_NextLoopIndex) "Local")))
      (LocalVariables|SetLocal_EndTangent (.Tangent (Spline|GetLocationandTangentatSplinePoint (Variables|Default|GetRoadSpline) (LocalVariables|GetLocal_NextLoopIndex) "Local")))
      ;[1 1 1] Set_StartBank/Roll
      (LocalVariables|SetLocal_StartRoll (.trackbank (Utilities|Array|Get(acopy) (Variables|Default|GetRoadDataArray) (LocalVariables|GetLocal_CurrentLoopIndex))))
      (LocalVariables|SetLocal_StartScale (Math|Vector2D|MakeVector2D (.trackwidth (Utilities|Array|Get(acopy) (Variables|Default|GetRoadDataArray) (LocalVariables|GetLocal_CurrentLoopIndex))) (.trackthickness (Utilities|Array|Get(acopy) (Variables|Default|GetRoadDataArray) (LocalVariables|GetLocal_CurrentLoopIndex)))))
      ;[1 1 1] Set_EndBank/Roll
      (LocalVariables|SetLocal_EndRoll (.trackbank (Utilities|Array|Get(acopy) (Variables|Default|GetRoadDataArray) (LocalVariables|GetLocal_NextLoopIndex))))
      (LocalVariables|SetLocal_EndScale (Math|Vector2D|MakeVector2D (.trackwidth (Utilities|Array|Get(acopy) (Variables|Default|GetRoadDataArray) (LocalVariables|GetLocal_NextLoopIndex))) (.trackthickness (Utilities|Array|Get(acopy) (Variables|Default|GetRoadDataArray) (LocalVariables|GetLocal_NextLoopIndex))))))
    (:then_1
      (bind _returnvalue (AddComponent|AddSplineMeshComponent false))
      (LocalVariables|SetLocal_CurrentSplineMesh _returnvalue)
      (Components|StaticMesh|SetStaticMesh (LocalVariables|GetLocal_CurrentSplineMesh) (LocalVariables|GetLocal_TrackElements))
      (SplineMesh|SetStartandEnd (LocalVariables|GetLocal_CurrentSplineMesh) (LocalVariables|GetLocal_StartLocation) (LocalVariables|GetLocal_StartTangent) (LocalVariables|GetLocal_EndLocation) (LocalVariables|GetLocal_EndTangent) true :!class /Script/Engine.SplineMeshComponent)
      (Class|SplineMeshComponent|SetStartRoll (LocalVariables|GetLocal_CurrentSplineMesh) (LocalVariables|GetLocal_StartRoll) true)
      (Class|SplineMeshComponent|SetEndRoll (LocalVariables|GetLocal_CurrentSplineMesh) (LocalVariables|GetLocal_EndRoll) true)
      ;[1 1 1] Set_Scale
      (SplineMesh|SetStartScale (LocalVariables|GetLocal_CurrentSplineMesh) (LocalVariables|GetLocal_StartScale) true :!class /Script/Engine.SplineMeshComponent)
      (SplineMesh|SetEndScale (LocalVariables|GetLocal_CurrentSplineMesh) (LocalVariables|GetLocal_EndScale) true :!class /Script/Engine.SplineMeshComponent)
      ;[1 1 1] Set_Collision
      (Collision|SetCollisionEnabled (LocalVariables|GetLocal_CurrentSplineMesh) (select (Variables|Default|GetMesh%20Collision) "QueryAndPhysics" "NoCollision")))))