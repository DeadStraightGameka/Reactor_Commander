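; Enemy tower turret that tracks player 0 and fires EnemyPojecttile_BP from its Bone003 socket about once a second while the player is in range.
; Tick drives everything: it feeds player-facing yaw and a distance-based pitch into Tower_Anim to aim the bone.
; The resulting angle is reused as the projectile's spawn roll, with yaw taken from the socket.
; A debug-drawn line trace precedes each shot, but both outcomes spawn the same projectile.
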(event EventBeginPlay)

(event Collision|EventActorBeginOverlap
  (params (OtherActor :type Actor%20Object%20Reference)))

(event EventTick
  (params (DeltaSeconds :type Float%20%28single-precision%29))
  (bind _returnvalue (Game|GetPlayerCharacter 0))
  (bind _self self)
  (bind _turret (Variables|Default|GetTurret))
  (bind _turret_2 (Variables|Default|GetTurret))
  (bind _turret_3 (Variables|Default|GetTurret))
  (bind _turret_4 (Variables|Default|GetTurret))
  (bind _returnvalue_2 (Transformation|GetWorldRotation _turret))
  (bind _returnvalue_3 (Transformation|GetSocketLocation _turret_2 "Bone003"))
  (bind _returnvalue_4 (Transformation|GetDistanceTo _self _returnvalue))
  (bind _returnvalue_5 (Transformation|GetSocketTransform _turret_3 "Bone003" "RTS_World"))
  (bind _returnvalue_6 (Transformation|GetSocketTransform _turret_4 "Bone003" "RTS_World"))
  (Utilities|FlowControl|Sequence
    (:then_0
      (if (Variables|Default|GetShootAble)
        (bind _output_get (Variables|Default|SetDelay%20Time (+ (Utilities|Time|GetWorldDeltaSeconds) (Variables|Default|GetDelay%20Time))))
        (if (>= _output_get 1.0)
          (bind _returnvalue_7 (Collision|LineTraceByChannel _returnvalue_3 (* _returnvalue_3 (* (Math|Vector|GetForwardVector (Transformation|GetWorldRotation _turret_2)) 5e+04)) "TraceTypeQuery1" false 0 "ForDuration"))
          (if _returnvalue_7
            (Game|SpawnActorfromClass "/Game/HP_Test_Folder/Blueprints/AI_Enemy/EnemyPojecttile_BP.EnemyPojecttile_BP_C" (Math|Transform|MakeTransform (.location _returnvalue_5) (Math|Rotator|MakeRotator (Variables|Default|GetCurrentAngle) 0.0 (- (.Yaw (Math|Rotator|BreakRotator (.rotation _returnvalue_5))) 9e+01)) "1,1,1") "AlwaysSpawn" 0 self)
            (else
              (Game|SpawnActorfromClass "/Game/HP_Test_Folder/Blueprints/AI_Enemy/EnemyPojecttile_BP.EnemyPojecttile_BP_C" (Math|Transform|MakeTransform (.location _returnvalue_6) (Math|Rotator|MakeRotator (Variables|Default|GetCurrentAngle) 0.0 (- (.Yaw (Math|Rotator|BreakRotator (.rotation _returnvalue_6))) 9e+01)) "1,1,1") "AlwaysSpawn" 0 self)))
          (Variables|Default|SetDelay%20Time 0.0))))
    (:then_1
      (bind _astower_anim (Utilities|Casting|CastToTower_Anim (Components|SkeletalMesh|GetAnimInstance (Variables|Default|GetTurret))))
      (bind _output_get_2 (Variables|/Game/HP_Test_Folder/Tower_Turret/Tower_Anim.Tower_Anim_C|SetRotation _astower_anim (Math|Rotator|MakeRotator (+ (.pitch _returnvalue_2) (Variables|Default|GetPitch_Angle)) 0.0 (- (* (- (.yaw _returnvalue_2) (.yaw (Math|Rotator|FindLookatRotation (Transformation|GetActorLocation self) (Transformation|GetActorLocation (Game|GetPlayerCharacter 0))))) -1.0) 9e+01))))
      (Variables|Default|SetCurrentAngle (.roll _output_get_2)))
    (:then_2
      (if (<= (Transformation|GetDistanceTo self (Game|GetPlayerCharacter 0)) 5e+03)
        (Variables|Default|SetShootAble true)
        (else
          (Variables|Default|SetShootAble false))))
    (:then_3
      (if (>= _returnvalue_4 2.5e+03)
        (if (<= _returnvalue_4 5e+03)
          (Variables|Default|SetPitch_Angle (- 5e+01 (/ _returnvalue_4 1e+02)))
          (else
            (Variables|Default|SetPitch_Angle 0.0)))
        (else
          (Variables|Default|SetPitch_Angle 25.0))))))

(fn ConstructionScript)