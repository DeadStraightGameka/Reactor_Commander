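; EnemyTower_BP is an enemy turret that tracks the player and fires projectiles while the player is within range.
; Each Tick updates the range flag, and a delay accumulator spawns EnemyPojecttile_BP from the Bone003 socket about once a second.
; A debug-drawn line trace runs before each shot, but both outcomes spawn the same projectile.
; Aiming feeds a look-at yaw toward the player into the Tower_Anim instance's Rotation.
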(event EventBeginPlay)

(event Collision|EventActorBeginOverlap
  (params (OtherActor :type Actor%20Object%20Reference)))

(event EventTick
  (params (DeltaSeconds :type Float%20%28single-precision%29))
  (bind _turret (Variables|Default|GetTurret))
  (bind _turret_2 (Variables|Default|GetTurret))
  (bind _turret_3 (Variables|Default|GetTurret))
  (bind _returnvalue (Transformation|GetSocketLocation _turret "GunHead"))
  (bind _returnvalue_2 (Transformation|GetSocketTransform _turret_2 "Bone003" "RTS_World"))
  (bind _returnvalue_3 (Transformation|GetSocketTransform _turret_3 "Bone003" "RTS_World"))
  (bind (_roll _pitch _yaw) (Math|Rotator|BreakRotator (.rotation _returnvalue_2)))
  (bind (_roll_2 _pitch_2 _yaw_2) (Math|Rotator|BreakRotator (.rotation _returnvalue_3)))
  (Utilities|FlowControl|Sequence
    (:then_0
      (if (Variables|Default|GetShootAble)
        (bind _output_get (Variables|Default|SetDelay%20Time (+ (Utilities|Time|GetWorldDeltaSeconds) (Variables|Default|GetDelay%20Time))))
        (if (>= _output_get 1.0)
          (bind _returnvalue_4 (Collision|LineTraceByChannel _returnvalue (* _returnvalue (* (Math|Vector|GetForwardVector (Transformation|GetWorldRotation _turret)) 5e+04)) "TraceTypeQuery1" false 0 "ForDuration"))
          (if _returnvalue_4
            (Game|SpawnActorfromClass "/Game/HP_Test_Folder/Blueprints/EnemyPojecttile_BP.EnemyPojecttile_BP_C" (Math|Transform|MakeTransform (.location _returnvalue_2) (Math|Rotator|MakeRotator _roll _pitch (- _yaw 9e+01)) "1,1,1") "AlwaysSpawn" 0 self)
            (else
              (Game|SpawnActorfromClass "/Game/HP_Test_Folder/Blueprints/EnemyPojecttile_BP.EnemyPojecttile_BP_C" (Math|Transform|MakeTransform (.location _returnvalue_3) (Math|Rotator|MakeRotator _roll_2 _pitch_2 (- _yaw_2 9e+01)) "1,1,1") "AlwaysSpawn" 0 self)))
          (Variables|Default|SetDelay%20Time 0.0))))
    (:then_1
      (bind _astower_anim (Utilities|Casting|CastToTower_Anim (Components|SkeletalMesh|GetAnimInstance (Variables|Default|GetTurret))))
      (Variables|/Game/HP_Test_Folder/Test_Turret/Tower_Anim.Tower_Anim_C|SetRotation _astower_anim (Math|Rotator|MakeRotator 0.0 0.0 (- (* (- (.yaw (Transformation|GetWorldRotation (Variables|Default|GetTurret))) (.yaw (Math|Rotator|FindLookatRotation (Transformation|GetActorLocation self) (Transformation|GetActorLocation (Game|GetPlayerCharacter 0))))) -1.0) 9e+01))))
    (:then_2
      (if (<= (Transformation|GetDistanceTo self (Game|GetPlayerCharacter 0)) 5e+03)
        (Variables|Default|SetShootAble true)
        (else
          (Variables|Default|SetShootAble false))))))

(fn ConstructionScript)