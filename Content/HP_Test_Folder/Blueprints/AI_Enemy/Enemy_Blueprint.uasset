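; Enemy AI character that chases the player and fires projectiles when within range.
; Each tick, distance to the player toggles between moving toward them and a combat mode that stops and fires EnemyPojecttile_BP once a second.
; A gun-head line trace precedes each shot, but both results spawn the same projectile.
; Tick also feeds the player-relative yaw to EnemyHead_AnimBP to aim the head.
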(event Collision|EventActorBeginOverlap
  (params (OtherActor :type Actor%20Object%20Reference)))

(event EventTick
  (params (DeltaSeconds :type Float%20%28single-precision%29))
  (bind _box002 (Variables|Default|GetBox002))
  (bind _returnvalue (Transformation|GetSocketLocation _box002 "GunHead"))
  (Utilities|FlowControl|Sequence
    (:then_0
      ;[1 1 1] Switch combat or moving mode
      (if (>= (Transformation|GetDistanceTo (Game|GetPlayerCharacter 0)) 2e+03)
        (Variables|Default|SetCombatMode false)
        (Variables|Default|SetMovingMode true)
        (else
          (Variables|Default|SetCombatMode true)
          (Variables|Default|SetMovingMode false))))
    (:then_1
      (if (Variables|Default|GetMovingMode)
        (AI|Navigation|SimpleMovetoActor (Pawn|GetController) (Game|GetPlayerCharacter 0))))
    (:then_2
      ;[1 1 1] Shoot
      (if (Variables|Default|GetCombatMode)
        (AI|Navigation|StopMovement (Pawn|GetController))
        (bind _output_get (Variables|Default|SetDelayTime (+ (Utilities|Time|GetWorldDeltaSeconds) (Variables|Default|GetDelayTime))))
        (if (>= _output_get 1.0)
          (bind _returnvalue_2 (Collision|LineTraceByChannel _returnvalue (* _returnvalue (* (Math|Vector|GetForwardVector (Transformation|GetWorldRotation _box002)) 5e+04)) "TraceTypeQuery1" false 0 "ForDuration"))
          (if _returnvalue_2
            (Game|SpawnActorfromClass "/Game/HP_Test_Folder/Blueprints/AI_Enemy/EnemyPojecttile_BP.EnemyPojecttile_BP_C" (Transformation|GetSocketTransform (Variables|Default|GetBox002) "Box002" "RTS_World") "AlwaysSpawn" 0 self)
            (else
              (Game|SpawnActorfromClass "/Game/HP_Test_Folder/Blueprints/AI_Enemy/EnemyPojecttile_BP.EnemyPojecttile_BP_C" (Transformation|GetSocketTransform (Variables|Default|GetBox002) "Box002" "RTS_World") "AlwaysSpawn" 0 self)))
          (Variables|Default|SetDelayTime 0.0))))
    (:then_3
      (bind _asenemy_head_anim_bp (Utilities|Casting|CastToEnemyHead_AnimBP (Components|SkeletalMesh|GetAnimInstance (Variables|Default|GetBox002))))
      (Variables|/Game/HP_Test_Folder/Blueprints/AI_Enemy/EnemyHead_AnimBP.EnemyHead_AnimBP_C|SetRotation _asenemy_head_anim_bp (Math|Rotator|MakeRotator 0.0 0.0 (* (- (.yaw (Transformation|GetWorldRotation (Variables|Collision|GetCapsuleComponent))) (.yaw (Math|Rotator|FindLookatRotation (Transformation|GetActorLocation self) (Transformation|GetActorLocation (Game|GetPlayerCharacter 0))))) -1.0))))))

(fn ConstructionScript)