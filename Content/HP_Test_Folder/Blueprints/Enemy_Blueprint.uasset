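; Enemy that chases the player when far away and stops to shoot when within range.
; Tick prints the player distance, sets moving or combat mode from it, then either calls SimpleMoveToActor or halts and fires once a timer fills.
; Each shot traces from the GunHead socket, with the end multiplying rather than adding the forward offset, and spawns EnemyPojecttile_BP facing the hit, or the gun's rotation on a miss.
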(event Collision|EventActorBeginOverlap
  (params (OtherActor :type Actor%20Object%20Reference)))

(event EventTick
  (params (DeltaSeconds :type Float%20%28single-precision%29))
  (bind _returnvalue (Game|GetPlayerCharacter 0))
  (bind _box002 (Variables|Default|GetBox002))
  (bind _returnvalue_2 (Transformation|GetWorldRotation _box002))
  (bind _returnvalue_3 (Transformation|GetSocketTransform _box002 "GunHead" "RTS_World"))
  (bind _returnvalue_4 (Transformation|GetSocketLocation _box002 "GunHead"))
  (bind _returnvalue_5 (Transformation|GetDistanceTo _returnvalue))
  (bind _location (Math|Transform|BreakTransform _returnvalue_3))
  (Utilities|FlowControl|Sequence
    (:then_0
      (Development|PrintString (Utilities|String|ToString(Float) _returnvalue_5))
      ;[1 1 1] Switch combat or moving mode
      (if (>= _returnvalue_5 2e+03)
        (Variables|Default|SetCombatMode false)
        (Variables|Default|SetMovingMode true)
        (else
          (Variables|Default|SetCombatMode true)
          (Variables|Default|SetMovingMode false))))
    (:then_1
      (if (Variables|Default|GetMovingMode)
        (AI|Navigation|SimpleMovetoActor (Pawn|GetController) (Game|GetPlayerCharacter 0))))
    (:then_2
      ;[1 1 1] Shoot
      (if (Variables|Default|GetCombatMode)
        (AI|Navigation|StopMovement (Pawn|GetController))
        (bind _output_get (Variables|Default|SetDelayTime (+ (Utilities|Time|GetWorldDeltaSeconds) (Variables|Default|GetDelayTime))))
        (if (>= _output_get 1.0)
          (bind (_outhit _returnvalue_6) (Collision|LineTraceByChannel _returnvalue_4 (* _returnvalue_4 (* (Math|Vector|GetForwardVector _returnvalue_2) 5e+04)) "TraceTypeQuery1" false 0 "ForDuration"))
          (if _returnvalue_6
            (Game|SpawnActorfromClass "/Game/HP_Test_Folder/Blueprints/EnemyPojecttile_BP.EnemyPojecttile_BP_C" (Math|Transform|MakeTransform _location (Math|Rotator|FindLookatRotation _location (.Location (Collision|BreakHitResult _outhit)))) "AlwaysSpawn" 0 self)
            (else
              (Game|SpawnActorfromClass "/Game/HP_Test_Folder/Blueprints/EnemyPojecttile_BP.EnemyPojecttile_BP_C" (Math|Transform|MakeTransform _location _returnvalue_2) "AlwaysSpawn" 0 self)))
          (Variables|Default|SetDelayTime 0.0))))))

(fn ConstructionScript)